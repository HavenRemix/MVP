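; Player pawn that owns the main HUD and drives its dynamic crosshair spread.
; On BeginPlay, only a locally controlled pawn creates the HUD widget, stores a reference and adds it to the viewport.
; Every Tick maps velocity magnitude to crosshair spread with a clamped range, or collapses it to zero while zooming.
; Tick writes through the HUD reference without a validity or local-control check.
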(event `self.ReceiveTick`
  (params (DeltaSeconds :type "Float (single-precision)"))
  ;[0 0 1] Crosshair Spread
  (if (`self.bWantsToZoom`)
    (set `/Game/UI/Combat/DynamicCrossHair.crosshair_spread` 0.0 (`/Game/UI/HUD/WBP_MainHUD.WBCrosshair` (`self.HUDRef`)))
    (else
      (set `/Game/UI/Combat/DynamicCrossHair.crosshair_spread` (`KismetMathLibrary.MapRangeClamped` (`KismetMathLibrary.VSize` (`self.GetVelocity`)) 0.0 600.0 20.0 80.0) (`/Game/UI/HUD/WBP_MainHUD.WBCrosshair` (`self.HUDRef`))))))

(event `self.ReceiveBeginPlay`
  (if (`self.IsLocallyControlled`)
    (bind _returnvalue (`|CreateWidget` "/Game/UI/HUD/WBP_MainHUD.WBP_MainHUD_C"))
    (bind _output_get (set `self.HUDRef` _returnvalue))
    (`UserWidget.AddToViewport` _output_get 0)))

(fn `UserConstructionScript`)