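; BP_TimedCollisionBlock is a block that alternates between a solid, visible state and a non-colliding outline state.
; Each Tick flips the State flag, swapping visibility between MeshComp and Border and switching MeshComp collision on or off.
; Border has its collision disabled at BeginPlay, so it never blocks.
; The graph has no timer, so the switching rate follows the actor's tick rate.
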(event `self.ReceiveBeginPlay`
  (`PrimitiveComponent.SetCollisionEnabled` (`self.Border`) "NoCollision"))

(event `self.ReceiveTick`
  (params (DeltaSeconds :type "Float (single-precision)"))
  (if (`self.State`)
    ;[1 0.9639 0] Visibility
    (`SceneComponent.SetVisibility` (`self.MeshComp`) true false)
    (`SceneComponent.SetVisibility` (`self.Border`) false false)
    (set `self.State` false)
    ;[0.1349 1 0] Collision
    (`PrimitiveComponent.SetCollisionEnabled` (`self.MeshComp`) "QueryAndPhysics")
    (else
      (`SceneComponent.SetVisibility` (`self.MeshComp`) false false)
      (`SceneComponent.SetVisibility` (`self.Border`) true false)
      (set `self.State` true)
      (`PrimitiveComponent.SetCollisionEnabled` (`self.MeshComp`) "NoCollision"))))

(fn `UserConstructionScript`)